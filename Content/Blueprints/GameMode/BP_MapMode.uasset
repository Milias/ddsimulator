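; BP_MapMode is a game mode that sets up a grid-based map and assigns the map HUD to joining players.
; On BeginPlay it calls ServerCreateBaseMap, then builds a basic 15x15 grid at the world origin through the Map on the MapState game state.
; PostLogin sets BP_MapHUD on each new player.
; An unconnected fragment that moves a tile's first assigned entity never runs.
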(event `self.ReceiveBeginPlay`
  (`self.ServerCreateBaseMap`)
  (bind _asmap_state (cast `MapState` (`GameplayStatics.GetGameState`)))
  (`MapBase.CreateBasicGridMap` (`MapState.Map` _asmap_state) (0.0 0.0 0.0) 15 15))

(event `self.K2_PostLogin`
  (params (NewPlayer :type "PlayerController Object Reference"))
  (`PlayerController.ClientSetHUD` NewPlayer "/Game/Blueprints/HUD/Map/BP_MapHUD.BP_MapHUD_C"))

(fn `UserConstructionScript`)