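; Map HUD Blueprint that manages the entity selection and action widgets for the owning player.
; Its construction script calls SetupHUD, which creates both widgets, adds them to the player screen and starts the actions panel hidden.
; UpdateSelection passes selected entities to both widgets and clears the MovingEntity flag.
; MoveEntityEvent only toggles that flag.
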(event `self.UpdateSelection`
  (params (SelectedEntities :type "Array of MapBasicEntity Object Reference (by ref)"))
  (`/Game/Blueprints/HUD/Map/BP_Selection.UpdateSelectedEntities` (`self.SelectionWidget`) SelectedEntities)
  (`/Game/Blueprints/HUD/Map/BP_Actions.UpdateActionLabels` (`self.ActionsWidget`) SelectedEntities)
  (set `self.MovingEntity` false))

(event `MoveEntityEvent`
  (set `self.MovingEntity` (not (`self.MovingEntity`))))

(fn `SetupHUD`
  (bind _returnvalue (`self.GetOwningPlayerController`))
  (bind _returnvalue_2 (`|CreateWidget` "/Game/Blueprints/HUD/Map/BP_Selection.BP_Selection_C" _returnvalue))
  (bind _output_get (set `self.SelectionWidget` _returnvalue_2))
  (`UserWidget.AddToPlayerScreen` _output_get 0)
  (bind _returnvalue_3 (`|CreateWidget` "/Game/Blueprints/HUD/Map/BP_Actions.BP_Actions_C" _returnvalue))
  (bind _output_get_2 (set `self.ActionsWidget` _returnvalue_3))
  (`UserWidget.AddToPlayerScreen` _output_get_2 0)
  (`Widget.SetVisibility` (`/Game/Blueprints/HUD/Map/BP_Actions.ScreenPanel` _output_get_2) "Hidden"))

(fn `UserConstructionScript`
  (`self.SetupHUD`))