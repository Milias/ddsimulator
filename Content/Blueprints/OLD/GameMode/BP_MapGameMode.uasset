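; Game mode that spawns the map grid when play begins and logs player logins.
; BeginPlay calls CreateMapGrid, which spawns a game-mode-owned BP_MapGrid with a fixed map and tile size.
; A NewPlayer function, not called in this graph, creates a local player without a pawn and stores it in Players.
; PreLogin and PostLogin only print debug text, and a tile-lookup debug print is left disconnected.
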(event `self.ReceiveBeginPlay`
  (bind _mapgrid (`self.CreateMapGrid` 20 20)))

(event `self.K2_PostLogin`
  (params (NewPlayer :type "PlayerController Object Reference"))
  (`KismetSystemLibrary.PrintString` (`KismetSystemLibrary.GetDisplayName` NewPlayer)))

(event `PreLogin`
  (`KismetSystemLibrary.PrintString` "PreLogin"))

(fn `CreateMapGrid`
  (params (MapWidth :type Integer) (MapHeight :type Integer))
  (returns (MapGrid :type "/Game/Blueprints/OLD/Map/BP_MapGrid Object Reference"))
  (bind _returnvalue (`|SpawnActorFromClass` "/Game/Blueprints/OLD/Map/BP_MapGrid.BP_MapGrid_C" (`KismetMathLibrary.MakeTransform` (0.0 0.0 0.0)) true self 250.0 250.0 MapWidth MapHeight))
  (return _returnvalue))

(fn `NewPlayer`
  (params (PlayerID :type Integer))
  (returns (Player :type "PlayerController Object Reference"))
  (bind _returnvalue (`GameplayStatics.CreatePlayer` PlayerID false))
  (`KismetArrayLibrary.Array_Add` (`self.Players`) _returnvalue)
  (return _returnvalue))

(fn `UserConstructionScript`)