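; BP_Map is a map Blueprint that provides coordinate-based lookup into a grid of tiles.
; GetTile clamps out-of-range I and J to the nearest edge or corner through nested branches, then passes them to GetTileFromIndex.
; GetTileFromIndex reads the flat MapTiles array at J + MapHeight * I, so tiles sharing an I are contiguous.
; BeginPlay and the construction script are empty, so these graphs never populate the array.
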(event EventBeginPlay)

(fn ConstructionScript)

(fn GetTile
  (params (I :type Integer) (J :type Integer))
  (bind _returnvalue (< J 0))
  (bind _returnvalue_2 (< I 0))
  (bind _mapwidth (Variables|Map|GetMapWidth))
  (bind _mapheight (Variables|Map|GetMapHeight))
  (bind _returnvalue_3 (>= J _mapheight))
  (bind _returnvalue_4 (>= I _mapwidth))
  (bind _returnvalue_5 (- _mapwidth 1))
  (bind _returnvalue_6 (- _mapheight 1))
  (if (and _returnvalue_4 _returnvalue_3)
    (bind _tile (CallFunction|GetTilefromIndex _returnvalue_5 _returnvalue_6))
    (LocalVariables|SetTempTile _tile)
    (elif (and _returnvalue_4 _returnvalue)
      (bind _tile_2 (CallFunction|GetTilefromIndex _returnvalue_5))
      (LocalVariables|SetTempTile _tile_2)
      (elif (and _returnvalue_2 _returnvalue_3)
        (bind _tile_3 (CallFunction|GetTilefromIndex 0 _returnvalue_6))
        (LocalVariables|SetTempTile _tile_3)
        (elif (and _returnvalue_2 _returnvalue)
          (bind _tile_4 (CallFunction|GetTilefromIndex))
          (LocalVariables|SetTempTile _tile_4)
          (elif _returnvalue_4
            (bind _tile_5 (CallFunction|GetTilefromIndex _returnvalue_5 J))
            (LocalVariables|SetTempTile _tile_5)
            (elif _returnvalue_2
              (bind _tile_6 (CallFunction|GetTilefromIndex 0 J))
              (LocalVariables|SetTempTile _tile_6)
              (elif _returnvalue_3
                (bind _tile_7 (CallFunction|GetTilefromIndex I _returnvalue_6))
                (LocalVariables|SetTempTile _tile_7)
                (elif _returnvalue
                  (bind _tile_8 (CallFunction|GetTilefromIndex I))
                  (LocalVariables|SetTempTile _tile_8)
                  (else
                    (bind _tile_9 (CallFunction|GetTilefromIndex I J))
                    (LocalVariables|SetTempTile _tile_9))))))))))
  (return (LocalVariables|GetTempTile)))

(fn GetTilefromIndex
  (params (I :type Integer) (J :type Integer))
  (return (Utilities|Array|Get(acopy) (Variables|Map|GetMapTiles) (+ J (* (Variables|Map|GetMapHeight) I)))))