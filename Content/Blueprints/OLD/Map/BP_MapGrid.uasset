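; BP_MapGrid is a map actor that builds a MapWidth by MapHeight grid of tiles centered on its origin.
; Its construction script clears MapTiles, then adds a BasicTile static mesh component per cell, spaced by TileWidth and TileHeight on a flat plane.
; Each cell is recorded in MapTiles as a BPMapTile holding its index, parent grid, mesh component and a WorldPosition set to the grid-relative offset.
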(fn `UserConstructionScript`
  (bind _tilewidth (`self.TileWidth`))
  (bind _tileheight (`self.TileHeight`))
  (bind _returnvalue (- (`self.MapHeight`) 1))
  (bind _returnvalue_2 (- (`self.MapWidth`) 1))
  (`KismetArrayLibrary.Array_Clear` (`self.MapTiles`))
  (for _index (range (+ _returnvalue_2 1))
    (for _index_2 (range (+ _returnvalue 1))
      (bind _returnvalue_3 (`KismetMathLibrary.MakeVector` (- (* (`KismetMathLibrary.Conv_IntToDouble` _index) _tilewidth) (* (/ (`KismetMathLibrary.Conv_IntToDouble` _returnvalue_2) 2.0) _tilewidth)) (- (* (`KismetMathLibrary.Conv_IntToDouble` _index_2) _tileheight) (* (/ (`KismetMathLibrary.Conv_IntToDouble` _returnvalue) 2.0) _tileheight))))
      (bind _returnvalue_4 (`AddComponent|Static Mesh Component_9` :`RelativeTransform` (`KismetMathLibrary.Conv_VectorToTransform` _returnvalue_3)))
      (`StaticMeshComponent.SetStaticMesh` _returnvalue_4 "/Game/Meshes/Basic/BasicTile.BasicTile")
      (`KismetArrayLibrary.Array_Add` (`self.MapTiles`) (make `/Game/Blueprints/OLD/Map/BP_MapTile` (`|MakeArray` _index _index_2) self _returnvalue_3 _returnvalue_4)))))