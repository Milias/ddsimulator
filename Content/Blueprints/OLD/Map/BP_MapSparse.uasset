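; Map actor Blueprint that builds a sparse tile map from an explicit list of tile positions.
; The construction script runs the parent script, then adds a static mesh component with the basic tile mesh at each 2D position, at zero height.
; It records each tile in MapTiles with its owner, world position, component and an index truncated directly from the position coordinates.
; The event graph holds no active logic.
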(event `self.ReceiveBeginPlay`)

(event `self.ReceiveActorBeginOverlap`
  (params (OtherActor :type "Actor Object Reference")))

(event `self.ReceiveTick`
  (params (DeltaSeconds :type "Float (single-precision)")))

(fn `UserConstructionScript`
  (`parent.UserConstructionScript`)
  (for _array_element (`self.MapTilePositions`)
    (bind _returnvalue (`KismetMathLibrary.MakeVector` (`KismetMathLibrary.BreakVector2D` _array_element) (`.Y` (`KismetMathLibrary.BreakVector2D` _array_element))))
    (bind _returnvalue_2 (`AddComponent|StaticMeshComponent_9` :`RelativeTransform` (`KismetMathLibrary.Conv_VectorToTransform` _returnvalue)))
    (`StaticMeshComponent.SetStaticMesh` _returnvalue_2 "/Game/Meshes/Basic/BasicTile.BasicTile")
    (`KismetArrayLibrary.Array_Add` (`self.MapTiles`) (make `/Game/Blueprints/OLD/Map/BP_MapTile` (`|MakeArray` (`KismetMathLibrary.FTrunc` (`KismetMathLibrary.BreakVector2D` _array_element)) (`KismetMathLibrary.FTrunc` (`.Y` (`KismetMathLibrary.BreakVector2D` _array_element)))) self _returnvalue _returnvalue_2))))